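; BP_PlayerPawn is the shooting game's player pawn, whose live logic only drives background scrolling.
; Tick accumulates time scaled by ScrollSpeed and writes it to the MPCBack material parameter collection, while key 1 increases that speed multiplicatively.
; BeginPlay creates a dynamic material on BP_Background, but its parameter write is disconnected.
; Movement, rotation, input mapping and timer nodes are also unwired.
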(event Custom|CustomEvent)

(event EventBeginPlay
  (bind _returnvalue (Actor|GetActorOfClass "/Game/Shooting/Blueprints/BP_Background.BP_Background_C"))
  (bind _returnvalue_2 (Rendering|Material|CreateDynamicMaterialInstance (Variables|/Script/Engine.StaticMeshActor|GetStaticMeshComponent _returnvalue) 0 (Rendering|Material|GetMaterial (Variables|/Script/Engine.StaticMeshActor|GetStaticMeshComponent _returnvalue) 0) "None" :!class /Script/Engine.PrimitiveComponent))
  (Variables|Default|SetBGMat _returnvalue_2))

(event Collision|EventActorBeginOverlap
  (params (OtherActor :type Actor%20Object%20Reference)))

(event EventTick
  (params (DeltaSeconds :type Float%20%28single-precision%29))
  (Variables|Default|SetScrollTime (+ (Variables|Default|GetScrollTime) (* DeltaSeconds (Variables|Default|GetScrollSpeed))))
  (Rendering|Material|SetScalarParameterValue (Variables|Default|GetMPC_Back) (Utilities|Name|MakeLiteralName "ScrollTime") (Variables|Default|GetScrollTime) :!class /Script/Engine.KismetMaterialLibrary))

(event Input|KeyboardEvents|1
  (params (Key :type Key%20Structure :default "None"))
  (:Pressed
    (Variables|Default|SetScrollSpeed (* (Variables|Default|GetScrollSpeed) 1.1))))

(fn ConstructionScript)